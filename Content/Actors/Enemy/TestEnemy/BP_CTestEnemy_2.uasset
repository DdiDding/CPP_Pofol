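; Test enemy character Blueprint that defers BeginPlay and Tick to its parent and prints the current character sub-state on screen every frame.
; GetUp ends ragdoll once when the character can get up and is in the DOWN state, re-arming otherwise, but nothing live calls it.
; Debug helpers for pelvis location and velocity, plus an upward launch, are also left disconnected.
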(event `self.ReceiveBeginPlay`
  (`parent.ReceiveBeginPlay`))

(event `self.ReceiveTick`
  (params (DeltaSeconds :type "Float (single-precision)"))
  (`parent.ReceiveTick` 0.0)
  (`|ExecutionSequence`
    (:`then_1`
      (`KismetSystemLibrary.PrintString` (`|GetEnumeratorNameAsString` (`CCharacterStruct.GetSubState` (`self.characterStructs`))) true false (struct :`G` 0.66 :`B` 1.0 :`A` 1.0) 0.0))))

(event `self.ReceiveAnyDamage`
  (params (Damage :type "Float (single-precision)") (DamageType :type "DamageType Object Reference") (InstigatedBy :type "Controller Object Reference") (DamageCauser :type "Actor Object Reference")))

(fn `UserConstructionScript`)