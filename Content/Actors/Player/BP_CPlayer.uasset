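; Player character Blueprint whose graphs hold developer debug and test hooks rather than gameplay logic.
; Hotkeys trigger ragdoll, a self-inflicted juggle hit, game instance calls, slow motion or freeze, speed multiplier tweaks, and debug toggles for wall running and weapons.
; A custom event creates an on-screen keyboard widget, with a helper graph for showing WASD and Space presses.
; Unwired leftover experiments cover friction, traces, camera shake and launches.
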(event `self.ReceiveTick`
  (params (DeltaSeconds :type "Float (single-precision)")))

(event `Key|T`
  (params (Key :type "Key Structure"))
  (:`Pressed`
    (`self.RagDollStart`)))

(event `Key|Y`
  (params (Key :type "Key Structure")))

(event `Key|U`
  (params (Key :type "Key Structure"))
  (:`Pressed`
    (`GameplayStatics.ApplyPointDamage` self 100.0 (0.0 0.0 0.0) (`GameplayStatics.MakeHitResult` true false 0.0 0.0 (0.0 0.0 0.0) (0.0 0.0 0.0) (0.0 0.0 1.0) (0.0 0.0 1.0) null self) null self "/Game/DataAsset/Skills/GreatSwordSkills/Combo_1/DT_GreatSword_Combo1_2.DT_GreatSword_Combo1_2_C")
    (`SkeletalMeshComponent.PlayAnimation` (`self.Mesh`) "/Game/Resources/Animaitions/Animation_HumanType/Hitted/InAir/A_Hitted_Juggle.A_Hitted_Juggle" false)
    (`CCharacterStruct.SetSubState_Hitted` (`self.characterStructs`))))

(event `키보드`
  ;[1 1 1] 키보드 디버깅
  (bind _returnvalue (`|CreateWidget` "/Game/Test_Code/keyboard.keyboard_C" (`GameplayStatics.GetPlayerController` 0)))
  (`UserWidget.AddToViewport` _returnvalue 0))

(event `Key|W`
  (params (Key :type "Key Structure"))
  ;[1 1 1] 키보드 디버깅
  (:`Pressed`
    (`/Engine/EditorBlueprintResources/StandardMacros.IsValid` (stale `키보드` _returnvalue)
      (:`Is Valid`
        (`/Game/Test_Code/keyboard.Press` (stale `키보드` _returnvalue) 0))))
  (:`Released`
    (`/Engine/EditorBlueprintResources/StandardMacros.IsValid` (stale `키보드` _returnvalue)
      (:`Is Valid`
        (`/Game/Test_Code/keyboard.Release` (stale `키보드` _returnvalue) 0)))))

(event `Key|A`
  (params (Key :type "Key Structure"))
  ;[1 1 1] 키보드 디버깅
  (:`Pressed`
    (`/Engine/EditorBlueprintResources/StandardMacros.IsValid` (stale `키보드` _returnvalue)
      (:`Is Valid`
        (`/Game/Test_Code/keyboard.Press` (stale `키보드` _returnvalue) 1))))
  (:`Released`
    (`/Engine/EditorBlueprintResources/StandardMacros.IsValid` (stale `키보드` _returnvalue)
      (:`Is Valid`
        (`/Game/Test_Code/keyboard.Release` (stale `키보드` _returnvalue) 1)))))

(event `Key|D`
  (params (Key :type "Key Structure"))
  ;[1 1 1] 키보드 디버깅
  (:`Pressed`
    (`/Engine/EditorBlueprintResources/StandardMacros.IsValid` (stale `키보드` _returnvalue)
      (:`Is Valid`
        (`/Game/Test_Code/keyboard.Press` (stale `키보드` _returnvalue) 3))))
  (:`Released`
    (`/Engine/EditorBlueprintResources/StandardMacros.IsValid` (stale `키보드` _returnvalue)
      (:`Is Valid`
        (`/Game/Test_Code/keyboard.Release` (stale `키보드` _returnvalue) 3)))))

(event `Key|S`
  (params (Key :type "Key Structure"))
  ;[1 1 1] 키보드 디버깅
  (:`Pressed`
    (`/Engine/EditorBlueprintResources/StandardMacros.IsValid` (stale `키보드` _returnvalue)
      (:`Is Valid`
        (`/Game/Test_Code/keyboard.Press` (stale `키보드` _returnvalue) 2))))
  (:`Released`
    (`/Engine/EditorBlueprintResources/StandardMacros.IsValid` (stale `키보드` _returnvalue)
      (:`Is Valid`
        (`/Game/Test_Code/keyboard.Release` (stale `키보드` _returnvalue) 2)))))

(event `Key|SpaceBar`
  (params (Key :type "Key Structure"))
  ;[1 1 1] 키보드 디버깅
  (:`Pressed`
    (`/Engine/EditorBlueprintResources/StandardMacros.IsValid` (stale `키보드` _returnvalue)
      (:`Is Valid`
        (`/Game/Test_Code/keyboard.Press` (stale `키보드` _returnvalue) 4))))
  (:`Released`
    (`/Engine/EditorBlueprintResources/StandardMacros.IsValid` (stale `키보드` _returnvalue)
      (:`Is Valid`
        (`/Game/Test_Code/keyboard.Release` (stale `키보드` _returnvalue) 4)))))

(event `self.ReceiveBeginPlay`
  (`|ExecutionSequence`
    (:`then_0`
      (set `CWallRunComponent.bDebugWallRun` false (`self.wallRunComponent`))
      (set `self.bOnDebugMode` false))))

(event `Key|K`
  (params (Key :type "Key Structure"))
  (:`Pressed`
    (bind _asbp_cgame_instance (cast `/Game/BP_CGameInstance` (`GameplayStatics.GetGameInstance`)))
    (`/Engine/EditorBlueprintResources/StandardMacros.IsValid` _asbp_cgame_instance
      (:`Is Valid`
        (`/Game/BP_CGameInstance.Press R` _asbp_cgame_instance)))))

(event `Key|L`
  (params (Key :type "Key Structure"))
  (:`Pressed`
    (bind _asbp_cgame_instance (cast `/Game/BP_CGameInstance` (`GameplayStatics.GetGameInstance`)))
    (`/Engine/EditorBlueprintResources/StandardMacros.IsValid` _asbp_cgame_instance
      (:`Is Valid`
        (`/Game/BP_CGameInstance.Press L` _asbp_cgame_instance)))))

(event `Key|Five`
  (params (Key :type "Key Structure"))
  (:`Pressed`
    (set `self.bOnDebugMode` (not (`self.bOnDebugMode`)))))

(event `Key|Six`
  (params (Key :type "Key Structure"))
  (bind _wallruncomponent (`self.wallRunComponent`))
  (:`Pressed`
    (set `CWallRunComponent.bDebugWallRun` (not (`CWallRunComponent.bDebugWallRun` _wallruncomponent)) _wallruncomponent)))

(event `Key|Eight`
  (params (Key :type "Key Structure"))
  (bind _weaponmanagercomponent8 (`self.weaponManagerComponent8`))
  (:`Pressed`
    (set `CWeaponManagerComponent.isDebugMode` (not (`CWeaponManagerComponent.isDebugMode` _weaponmanagercomponent8)) _weaponmanagercomponent8)))

(event `Key|X`
  (params (Key :type "Key Structure"))
  (:`Pressed`
    (`GameplayStatics.SetGlobalTimeDilation` 0.1))
  (:`Released`
    (`GameplayStatics.SetGlobalTimeDilation` 1.0)))

(event `Key|V`
  (params (Key :type "Key Structure"))
  (:`Pressed`
    (`GameplayStatics.SetGlobalTimeDilation` 0.0))
  (:`Released`
    (`GameplayStatics.SetGlobalTimeDilation` 1.0)))

(event `Key|Z`
  (params (Key :type "Key Structure"))
  (:`Pressed`
    (set `self.multiplySpeed` (+ (`self.multiplySpeed`) 0.1))))

(event `Key|C`
  (params (Key :type "Key Structure"))
  (:`Pressed`
    (set `self.multiplySpeed` (+ (`self.multiplySpeed`) -0.1))))

(fn `UserConstructionScript`)