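; BP_CGameInstance is a game instance Blueprint that provides level switching and a temporary per-object time freeze.
; SetTestCustomTime zeroes the passed object's CustomTimeDilation and starts a timer event that restores it to normal after the given delay.
; PressL advances a wrapping index through LevelArray and prints the selected level name, and PressR opens that level.
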(event `SetTestCustomTime`
  (params (NewParam :type "Actor Object Reference") (`delay time` :type "Float (double-precision)"))
  (`KismetSystemLibrary.K2_SetTimerDelegate` (delegate `test`) `delay time`)
  (set `Actor.CustomTimeDilation` 0.0 NewParam))

(event `test`
  (set `Actor.CustomTimeDilation` 1.0 (stale `SetTestCustomTime` NewParam)))

(event `Press R`
  (`GameplayStatics.OpenLevel` (`|GetArrayItem` (`self.LevelArray`) (`self.LevelIndex`))))

(event `Press L`
  (`/Engine/EditorBlueprintResources/StandardMacros.IncrementInt` (`self.LevelIndex`)
    (:`  `
      (if (== (`self.LevelIndex`) (`KismetArrayLibrary.Array_Length` (`self.LevelArray`)))
        (set `self.LevelIndex` 0))
      (`KismetSystemLibrary.PrintString` (`KismetStringLibrary.Concat_StrStr` "Move to " (`KismetStringLibrary.Conv_NameToString` (`|GetArrayItem` (`self.LevelArray`) (`self.LevelIndex`))))))))